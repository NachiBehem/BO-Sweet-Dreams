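; Werewolf enemy NPC that fights Alice with a three-hit montage combo, queuing follow-up swipes when attacks arrive mid-swing.
; Left and right box overlaps deal throttled damage, and another box flags Dream Eater availability on Alice.
; Looping fear timers drain player health: sight-based inside Fear_Sphere, plus a weaker hearing variant.
; Freeze events toggle a blackboard key and ice emitter; helpers handle scream anticipation and facing-angle block checks.
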(event `Anticipation`
  (`/Engine/EditorBlueprintResources/StandardMacros.DoOnce` false :!label _label
    (:`Completed`
      (`self.PlayAnimMontage` "/Game/AI/Werewolf/Animazioni/Zombie_Scream_Montage.Zombie_Scream_Montage")
      (if (not (`self.Spotted?`))
        (goto _label :!via `Reset`)))))

(event `Attack Player`
  ;[1 1 1] Attacking + Combos
  (if (`self.ReadyToAttack?`)
    (if (`self.Stunned`)
      _
      (elif (`self.Attacking?`)
        (set `self.SaveAttack` true)
        (else
          (set `self.Attacking?` true)
          (switch `int` (`self.AttackCount`) :!label _label_2
            (:`0`
              (set `self.AttackCount` 1)
              (`self.PlayAnimMontage` "/Game/AI/Werewolf/Animazioni/Mutant_Swiping_Montage.Mutant_Swiping_Montage"))
            (:`1`
              (set `self.AttackCount` 2)
              (`self.PlayAnimMontage` "/Game/AI/Werewolf/Animazioni/Mutant_Swiping__R__Montage.Mutant_Swiping__R__Montage"))
            (:`2`
              (set `self.AttackCount` 3)
              (`self.PlayAnimMontage` "/Game/AI/Werewolf/Animazioni/Mutant_Punch_Montage.Mutant_Punch_Montage"))))))))

(event `AttackCombo`
  ;[1 1 1] Attacking + Combos
  (if (`self.SaveAttack`)
    (set `self.SaveAttack` false)
    (if (== (`self.AttackCount`) 3)
      (`KismetSystemLibrary.Delay` 0.7)
      (else
        (goto _label_2))))
  (set `self.AttackCount` 0)
  (set `self.Attacking?` false))

(event `freezedOn`
  (bind _mesh (`self.Mesh`))
  ;[1 1 1] FreezeMode
  (`BlackboardComponent.SetValueAsBool` (`AIBlueprintHelperLibrary.GetBlackboard` null) "Freezed?" true)
  (bind _returnvalue (`GameplayStatics.SpawnEmitterAttached` "/Game/Luos8Elements/Particles/Ice/Par_4E_Ice_Def_01.Par_4E_Ice_Def_01" _mesh "None" (`SceneComponent.K2_GetComponentLocation` _mesh) (struct) (0.5 0.5 0.2) "KeepWorldPosition")))

(event `freezedOff`
  ;[1 1 1] FreezeMode
  (`BlackboardComponent.SetValueAsBool` (`AIBlueprintHelperLibrary.GetBlackboard` null) "Freezed?" false)
  (`ActorComponent.K2_DestroyComponent` (stale `freezedOn` _returnvalue)))

(event `self.Box_R.OnComponentBeginOverlap`
  (params (OverlappedComponent :type "PrimitiveComponent Object Reference") (OtherActor :type "Actor Object Reference") (OtherComp :type "PrimitiveComponent Object Reference") (OtherBodyIndex :type Integer) (bFromSweep :type Boolean) (SweepResult :type "HitResult Structure (by ref)"))
  ;[1 1 1] Deal Damage
  (bind _asalice (cast `/Game/Alice/Toon/Blueprints/Alice` (stale `self.Box_L.OnComponentBeginOverlap` OtherActor) :!label _label_3))
  (if (`self.AttackRdy_0`)
    (`/Engine/EditorBlueprintResources/StandardMacros.DoOnce` false :!label _label_4
      (:`Completed`
        (set `/Game/Alice/Toon/Blueprints/Alice.Hitted?` true _asalice)
        (`GameplayStatics.ApplyDamage` _asalice 10.0 null self)
        (`KismetSystemLibrary.Delay` 0.5)
        (goto _label_4 :!via `Reset`)))))

(event `self.Box_L.OnComponentBeginOverlap`
  (params (OverlappedComponent :type "PrimitiveComponent Object Reference") (OtherActor :type "Actor Object Reference") (OtherComp :type "PrimitiveComponent Object Reference") (OtherBodyIndex :type Integer) (bFromSweep :type Boolean) (SweepResult :type "HitResult Structure (by ref)"))
  ;[1 1 1] Deal Damage
  (goto _label_3))

(event `self.Dream_Eater_Box.OnComponentBeginOverlap`
  (params (OverlappedComponent :type "PrimitiveComponent Object Reference") (OtherActor :type "Actor Object Reference") (OtherComp :type "PrimitiveComponent Object Reference") (OtherBodyIndex :type Integer) (bFromSweep :type Boolean) (SweepResult :type "HitResult Structure (by ref)"))
  ;[1 1 1] Dream_Eater_Set
  (bind _asalice (cast `/Game/Alice/Toon/Blueprints/Alice` OtherActor))
  (set `/Game/Alice/Toon/Blueprints/Alice.Dream Eater Avaliable` true _asalice))

(event `self.Dream_Eater_Box.OnComponentEndOverlap`
  (params (OverlappedComponent :type "PrimitiveComponent Object Reference") (OtherActor :type "Actor Object Reference") (OtherComp :type "PrimitiveComponent Object Reference") (OtherBodyIndex :type Integer))
  ;[1 1 1] Dream_Eater_Set
  (bind _asalice (cast `/Game/Alice/Toon/Blueprints/Alice` OtherActor))
  (set `/Game/Alice/Toon/Blueprints/Alice.Dream Eater Avaliable` false _asalice))

(event `self.Fear_Sphere.OnComponentBeginOverlap`
  (params (OverlappedComponent :type "PrimitiveComponent Object Reference") (OtherActor :type "Actor Object Reference") (OtherComp :type "PrimitiveComponent Object Reference") (OtherBodyIndex :type Integer) (bFromSweep :type Boolean) (SweepResult :type "HitResult Structure (by ref)"))
  (if (`self.ActorHasTag` OtherActor "player")
    (if (`BlackboardComponent.GetValueAsBool` (`AIBlueprintHelperLibrary.GetBlackboard` null) "CanSeePlayer?")
      (bind _returnvalue (`KismetSystemLibrary.K2_SetTimerDelegate` (delegate `Paura_VIsta`) 2.0 true))
      (set `self.Timer_Vista` _returnvalue))))

(event `Paura_VIsta`
  (`GameplayStatics.ApplyDamage` (`GameplayStatics.GetPlayerCharacter` 0) 3.0 null self))

(event `Paura_Udito`
  (`GameplayStatics.ApplyDamage` (`GameplayStatics.GetPlayerCharacter` 0) 1.0 null self))

(event `TImer_Fear`
  (bind _returnvalue (`KismetSystemLibrary.K2_SetTimerDelegate` (delegate `Paura_Udito`) 1.0 true))
  (set `self.Timer_Udito` _returnvalue))

(event `self.Fear_Sphere.OnComponentEndOverlap`
  (params (OverlappedComponent :type "PrimitiveComponent Object Reference") (OtherActor :type "Actor Object Reference") (OtherComp :type "PrimitiveComponent Object Reference") (OtherBodyIndex :type Integer))
  (if (`self.ActorHasTag` OtherActor "player")
    (`KismetSystemLibrary.K2_ClearAndInvalidateTimerHandle` (`self.Timer_Vista`))))

(fn `BlockAngleCheck`
  (returns (FaceinAI :type Boolean))
  (bind (_returnvalue_roll _returnvalue_pitch _returnvalue_yaw) (`KismetMathLibrary.BreakRotator` (`self.K2_GetActorRotation`)))
  (bind (_returnvalue_roll_2 _returnvalue_pitch_2 _returnvalue_yaw_2) (`KismetMathLibrary.BreakRotator` (`self.K2_GetActorRotation` (`self.AttackingActor`))))
  (bind _returnvalue (- _returnvalue_yaw _returnvalue_yaw_2))
  (return (or (> _returnvalue 150.0) (< _returnvalue -150.0))))

(fn `UserConstructionScript`)