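; AshbringerNormalBP is a weapon the player character can pick up and use to deal melee damage.
; PickUp drops any equipped weapon at this one's transform, registers itself as EquippedWeapon and attaches to the character mesh's weapon_back socket.
; AttackRdy and AttackNoRdy toggle a flag that lets Box overlaps apply fixed damage to the overlapping actor.
; A DoOnce with a delayed reset limits how often hits land.
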(event `/Game/Ashbringers/WeaponPickupInterface.PickUp`
  (bind _defaultsceneroot (`self.DefaultSceneRoot`))
  (bind _asthird_person_character (cast `/Game/ThirdPersonBP/ThirdPersonCharacter` (`GameplayStatics.GetPlayerCharacter` 0) :!pure true))
  (bind _equippedweapon (`/Game/ThirdPersonBP/ThirdPersonCharacter.EquippedWeapon` _asthird_person_character))
  (`/Engine/EditorBlueprintResources/StandardMacros.IsValid` _equippedweapon
    (:`Is Valid`
      (`self.K2_DetachFromActor` _equippedweapon "KeepRelative" "KeepRelative" "KeepRelative")
      (`self.K2_SetActorLocationAndRotation` _equippedweapon (`SceneComponent.K2_GetComponentLocation` _defaultsceneroot) (`SceneComponent.K2_GetComponentRotation` _defaultsceneroot) false false))
    (:`Is Not Valid`
      _))
  (set `/Game/ThirdPersonBP/ThirdPersonCharacter.EquippedWeapon` self _asthird_person_character)
  (`self.K2_AttachToComponent` (`Character.Mesh` _asthird_person_character) "weapon_back" "SnapToTarget" "SnapToTarget" "KeepRelative"))

(event `self.Box.OnComponentBeginOverlap`
  (params (OverlappedComponent :type "PrimitiveComponent Object Reference") (OtherActor :type "Actor Object Reference") (OtherComp :type "PrimitiveComponent Object Reference") (OtherBodyIndex :type Integer) (bFromSweep :type Boolean) (SweepResult :type "HitResult Structure (by ref)"))
  ;[1 1 1] Deal Damage
  (if (`self.AttackRdy_0`)
    (`/Engine/EditorBlueprintResources/StandardMacros.DoOnce` false :!label _label
      (:`Completed`
        (`GameplayStatics.ApplyDamage` OtherActor 10.0)
        (`KismetSystemLibrary.Delay` 0.5)
        (goto _label :!via `Reset`)))))

(event `/Game/Ashbringers/WeaponPickupInterface.AttackRdy`
  (set `self.AttackRdy_0` true))

(event `/Game/Ashbringers/WeaponPickupInterface.AttackNoRdy`
  (set `self.AttackRdy_0` false))

(fn `UserConstructionScript`)