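; Piano minigame actor that takes over camera and input on player interaction and shows W_Piano with a track list.
; Key actions route by State: Practice plays notes on the child BP_PianoKeyboard, with held octave-shift modifiers.
; Track mode starts a track's Level Sequence, forwards keys to the child Audio_Processor_BP and scores matching registered falling notes.
; InitSound is empty; its synth setup is disconnected.
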(event `/Game/BaseIteractableInterface.On Player Interact`
  (params (Player :type "/Game/ThirdPersonBP/ThirdPersonCharacter Object Reference"))
  (bind _returnvalue (`GameplayStatics.GetPlayerController` 0))
  (bind _ui_ref (`self.UI REF`))
  ;[1 1 1] Open minigame
  (bind _output_get (set `self.Player REF` Player))
  (`/Game/ThirdPersonBP/ThirdPersonCharacter.Set Minigame Mode` _output_get true)
  (`self.EnableInput` _returnvalue)
  (`PlayerController.SetViewTargetWithBlend` _returnvalue self 1.0 "VTBlend_Linear" 0.0 false)
  (bind _returnvalue_2 (`|CreateWidget` "/Game/Piano_minigame/UI/W_Piano.W_Piano_C"))
  (`/Game/Piano_minigame/UI/W_Piano.SetPianoReference` _returnvalue_2 self)
  (bind _output_get_2 (set `self.UI REF` _returnvalue_2))
  (`UserWidget.AddToViewport` _returnvalue_2 0)
  (`UserWidget.AddToViewport` _output_get_2 0)
  (add `/Game/Piano_minigame/UI/W_Piano.OnClosePiano` _ui_ref (delegate `OnClosePiano`))
  (add `/Game/Piano_minigame/UI/W_Piano.OnStopTrack` _ui_ref (delegate `OnStopSong`))
  (`self.InitSound`)
  ;[1 1 1] Populate list of tracks
  (for _array_element (`self.Tracks`)
    (`/Game/Piano_minigame/UI/W_Piano.AddTrackToList` (`self.UI REF`) _array_element)))

(event `OnClosePiano`
  ;[1 1 1] Open minigame
  (`self.ClosePiano`))

(event `OnStopSong`
  ;[1 1 1] Open minigame
  (`self.StopTrack`))

(event `/Game/Piano_minigame/Blueprints/I_Piano.StartPlayTrack`
  (params (`Track data` :type "/Game/Piano_minigame/Blueprints/Data_Piano_Minigame_track Object Reference"))
  ;[1 1 1] MainGame events
  (bind _tracksequencer (`/Game/Piano_minigame/Blueprints/Data_Piano_Minigame_track.GetTrack` `Track data`))
  (bind _outactor (`LevelSequencePlayer.CreateLevelSequencePlayer` _tracksequencer))
  (`MovieSceneSequencePlayer.Play` (`LevelSequenceActor.SequencePlayer` _outactor))
  (set `self.State` "NewEnumerator2"))

(event `ClosePiano`
  (bind _returnvalue (`GameplayStatics.GetPlayerController` 0))
  (bind _player_ref (`self.Player REF`))
  ;[1 1 1] Close minigame
  (`/Game/ThirdPersonBP/ThirdPersonCharacter.Set Minigame Mode` _player_ref false)
  (`PlayerController.SetViewTargetWithBlend` _returnvalue _player_ref 1.0 "VTBlend_Linear" 0.0 false)
  (`Widget.RemoveFromParent` (`self.UI REF`))
  (`self.DisableInput` _returnvalue))

(event `StopTrack`
  ;[1 1 1] MainGame events
  (`/Game/Piano_minigame/Blueprints/Audio_Processor_BP.StopTrack` (`self.AudioProcessor_REF`))
  (set `self.State` "NewEnumerator0"))

(event `/Game/Piano_minigame/Blueprints/I_Piano.StartPractice`
  ;[1 1 1] PracticeEvents
  (set `self.State` "NewEnumerator1"))

(event `InputAction|Piano_C#`
  (params (Key :type "Key Structure"))
  ;[0.4452 0.5346 1] Piano keys C-E
  (:`Pressed`
    (`self.ProcessKeyInputPress` false 15))
  (:`Released`
    (`self.ProcessKeyInputRelease` 0)))

(event `InputAction|Piano_D#`
  (params (Key :type "Key Structure"))
  ;[0.4452 0.5346 1] Piano keys C-E
  (:`Pressed`
    (`self.ProcessKeyInputPress` false 16))
  (:`Released`
    (`self.ProcessKeyInputRelease` 0)))

(event `InputAction|Piano_E`
  (params (Key :type "Key Structure"))
  ;[0.4452 0.5346 1] Piano keys C-E
  (:`Pressed`
    (`self.ProcessKeyInputPress` true 23 2))
  (:`Released`
    (`self.ProcessKeyInputRelease` 2)))

(event `InputAction|Piano_D`
  (params (Key :type "Key Structure"))
  ;[0.4452 0.5346 1] Piano keys C-E
  (:`Pressed`
    (`self.ProcessKeyInputPress` true 22 1))
  (:`Released`
    (`self.ProcessKeyInputRelease` 1)))

(event `InputAction|Piano_C`
  (params (Key :type "Key Structure"))
  ;[0.4452 0.5346 1] Piano keys C-E
  (:`Pressed`
    (`self.ProcessKeyInputPress` true 21))
  (:`Released`
    (`self.ProcessKeyInputRelease` 0)))

(event `InputAction|Piano_F#`
  (params (Key :type "Key Structure"))
  ;[0.4452 0.5346 1] Piano keys F_B
  (:`Pressed`
    (`self.ProcessKeyInputPress` false 17))
  (:`Released`
    (`self.ProcessKeyInputRelease` 0)))

(event `InputAction|Piano_G#`
  (params (Key :type "Key Structure"))
  ;[0.4452 0.5346 1] Piano keys F_B
  (:`Pressed`
    (`self.ProcessKeyInputPress` false 18))
  (:`Released`
    (`self.ProcessKeyInputRelease` 0)))

(event `InputAction|Piano_A#`
  (params (Key :type "Key Structure"))
  ;[0.4452 0.5346 1] Piano keys F_B
  (:`Pressed`
    (`self.ProcessKeyInputPress` false 19))
  (:`Released`
    (`self.ProcessKeyInputRelease` 0)))

(event `InputAction|Piano_F`
  (params (Key :type "Key Structure"))
  ;[0.4452 0.5346 1] Piano keys F_B
  (:`Pressed`
    (`self.ProcessKeyInputPress` true 24 3))
  (:`Released`
    (`self.ProcessKeyInputRelease` 3)))

(event `InputAction|Piano_G`
  (params (Key :type "Key Structure"))
  ;[0.4452 0.5346 1] Piano keys F_B
  (:`Pressed`
    (`self.ProcessKeyInputPress` true 25 4))
  (:`Released`
    (`self.ProcessKeyInputRelease` 4)))

(event `InputAction|Piano_A`
  (params (Key :type "Key Structure"))
  ;[0.4452 0.5346 1] Piano keys F_B
  (:`Pressed`
    (`self.ProcessKeyInputPress` true 26 5))
  (:`Released`
    (`self.ProcessKeyInputRelease` 5)))

(event `InputAction|Piano_B`
  (params (Key :type "Key Structure"))
  ;[0.4452 0.5346 1] Piano keys F_B
  (:`Pressed`
    (`self.ProcessKeyInputPress` true 27 6))
  (:`Released`
    (`self.ProcessKeyInputRelease` 6)))

(event `InputAction|Piano_Lower`
  (params (Key :type "Key Structure"))
  ;[0.4452 0.5346 1] Lower and upper octaves
  (:`Pressed`
    (set `self.WhiteNoteModifier` -7)
    (set `self.BlackNoteModifier` -5))
  (:`Released`
    (set `self.WhiteNoteModifier` 0)
    (set `self.BlackNoteModifier` 0)))

(event `InputAction|Piano_Upper`
  (params (Key :type "Key Structure"))
  ;[0.4452 0.5346 1] Lower and upper octaves
  (:`Pressed`
    (set `self.WhiteNoteModifier` 7)
    (set `self.BlackNoteModifier` 5))
  (:`Released`
    (set `self.WhiteNoteModifier` 0)
    (set `self.BlackNoteModifier` 0)))

(event `/Game/Piano_minigame/Blueprints/I_Piano.FallingNoteEnter`
  (params (Note_Object :type "/Game/Piano_minigame/Blueprints/Falling_Note Object Reference"))
  ;[1 1 1] FallingNoteEvents
  (`KismetArrayLibrary.Array_Add` (`self.FallingNotes`) Note_Object)
  (set `self.TrackNoteCount` (+ (`self.TrackNoteCount`) 1) :!label _label))

(event `/Game/Piano_minigame/Blueprints/I_Piano.FallingNoteMiss`
  (params (NoteObject :type "/Game/Piano_minigame/Blueprints/Falling_Note Object Reference"))
  ;[1 1 1] FallingNoteEvents
  (`KismetArrayLibrary.Array_RemoveItem` (`self.FallingNotes`) NoteObject)
  (goto _label))

(fn `InitSound`
  (locals (NewLocalVar_0 :type "ChildActorComponent Object Reference")))

(fn `ProcessKeyInputPress`
  (params (IsWhiteKey :type Boolean) (KeyboardKeyId :type Integer) (TrackpadKeyId :type Integer))
  (bind _keyboardfull_ref (`self.KeyboardFull_REF`))
  (switch `/Game/Piano_minigame/Blueprints/EPiano_State` (`self.State`)
    (:`NewEnumerator1`
      (if IsWhiteKey
        (`/Game/Piano_minigame/Blueprints/BP_PianoKeyboard.Play Note` _keyboardfull_ref (+ KeyboardKeyId (`self.WhiteNoteModifier`)) "white")
        (else
          (`/Game/Piano_minigame/Blueprints/BP_PianoKeyboard.Play Note` _keyboardfull_ref (+ KeyboardKeyId (`self.BlackNoteModifier`)) "black"))))
    (:`NewEnumerator2`
      (`/Game/Piano_minigame/Blueprints/Audio_Processor_BP.Note Pressed` (`self.AudioProcessor_REF`) TrackpadKeyId)
      (for _array_element (`self.FallingNotes`)
        (if (== (`/Game/Piano_minigame/Blueprints/Falling_Note.Id` _array_element) TrackpadKeyId)
          (bind _score (`/Game/Piano_minigame/Blueprints/Falling_Note.PlayerHitNote` _array_element))
          (bind _output_get (set `self.Score` (+ _score (`self.Score`))))
          (`TextBlock.SetText` (`/Game/Piano_minigame/UI/W_Piano.txt_hitNote` (`self.UI REF`)) (`KismetTextLibrary.Conv_IntToText` _output_get)))))))

(fn `ProcessKeyInputRelease`
  (params (TrackpadKeyId :type Integer))
  (switch `/Game/Piano_minigame/Blueprints/EPiano_State` (`self.State`)
    (:`NewEnumerator2`
      (`/Game/Piano_minigame/Blueprints/Audio_Processor_BP.NoteReleased` (`self.AudioProcessor_REF`) TrackpadKeyId))))

(fn `UserConstructionScript`
  (bind _asbp_piano_keyboard (cast `/Game/Piano_minigame/Blueprints/BP_PianoKeyboard` (`ChildActorComponent.ChildActor` (`self.Piano_BP`))))
  (set `self.KeyboardFull_REF` _asbp_piano_keyboard)
  (bind _asaudio_processor_bp (cast `/Game/Piano_minigame/Blueprints/Audio_Processor_BP` (`ChildActorComponent.ChildActor` (`self.Audio_Processor_BP`))))
  (bind _output_get (set `self.AudioProcessor_REF` _asaudio_processor_bp))
  (set `/Game/Piano_minigame/Blueprints/Audio_Processor_BP.Piano_REF` self _output_get))