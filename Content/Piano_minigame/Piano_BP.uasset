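; Piano actor for a minigame that plays a sound and animates the matching key for each note.
; Construction script procedurally lays out octaves of white and black keys as two instanced static meshes.
; PlayNote triggers PlaySound, which tracks a capped list of recent sounds for StopSound and tilts the key instance through a timeline.
; A queue of pressed keys feeds a second, self-restarting timeline that rotates them back in turn.
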(event `self.StopSound`
  (bind _allpianosound (`self.AllPianoSound`))
  ;[1 1 1] Stop all sound
  (for _index (range (+ (`KismetArrayLibrary.Array_LastIndex` _allpianosound) 1))
    (bind _output (`|GetArrayItem` _allpianosound _index))
    (`/Engine/EditorBlueprintResources/StandardMacros.IsValid` _output
      (:`Is Valid`
        (`AudioComponent.Stop` _output)))))

(event `self.PlaySound`
  (params (Index :type Integer) (KeyType :type String))
  (bind _returnvalue (`self.K2_GetActorLocation`))
  (bind _allpianosound (`self.AllPianoSound`))
  (bind _returnvalue_2 (== (`KismetArrayLibrary.Array_LastIndex` _allpianosound) 10))
  ;[1 0.25 0.25] Play sound by pressing piano key
  (switch `string` KeyType
    (:`White`
      (bind _returnvalue_3 (`GameplayStatics.SpawnSoundAtLocation` (`|GetArrayItem` (`self.WhiteKeysSound`) Index) _returnvalue (struct) 1.0 1.0 0.0 null null))
      (`KismetArrayLibrary.Array_Add` _allpianosound _returnvalue_3)
      (if _returnvalue_2
        (`KismetArrayLibrary.Array_Remove` _allpianosound))
      (`self.Animation` (`self.WhiteKeysArray`) Index 10.0))
    (:`Black`
      (bind _returnvalue_4 (`GameplayStatics.SpawnSoundAtLocation` (`|GetArrayItem` (`self.BlackKeysSound`) Index) _returnvalue (struct) 1.0 1.0 0.0 null null))
      (`KismetArrayLibrary.Array_Add` _allpianosound _returnvalue_4)
      (if _returnvalue_2
        (`KismetArrayLibrary.Array_Remove` _allpianosound))
      (`self.Animation` (`self.BlackKeysArray`) Index 5.0))))

(event `Animation`
  (params (Key :type "Array of InstancedStaticMeshComponent Object Reference") (Index :type Integer) (Angle :type "Float (double-precision)"))
  (bind _output (`|GetArrayItem` Key Index))
  (bind _outinstancetransform (`InstancedStaticMeshComponent.GetInstanceTransform` _output Index false))
  ;[0.4062 0.4841 1] Piano keys animation
  (`KismetArrayLibrary.Array_Add` (`self.ActiveAnimation`) Index)
  (`KismetArrayLibrary.Array_Add` (`self.ActiveKey`) _output)
  (bind (_direction _alpha) (`Timeline|Rotator` :!via `PlayFromStart`)
    (:`Update`
      (`InstancedStaticMeshComponent.UpdateInstanceTransform` _output Index (`KismetMathLibrary.MakeTransform` (.location _outinstancetransform) (`KismetMathLibrary.MakeRotator` (`KismetMathLibrary.Lerp` (.roll (.rotation _outinstancetransform)) Angle _alpha)) (.scale _outinstancetransform)) false true false)
      (`self.CheckForActiveKey`))))

(event `CheckForActiveKey`
  (bind _output (`|GetArrayItem` (`self.ActiveKey`)))
  (bind _output_2 (`|GetArrayItem` (`self.ActiveAnimation`)))
  (bind _outinstancetransform (`InstancedStaticMeshComponent.GetInstanceTransform` _output _output_2 false))
  ;[0.4062 0.4841 1] Piano keys animation
  (if (!= (`KismetArrayLibrary.Array_Length` (`self.ActiveAnimation`)) 0)
    (bind (_direction _alpha) (`Timeline|BackRotator` :!via `PlayFromStart`)
      (:`Update`
        (`/Engine/EditorBlueprintResources/StandardMacros.IsValid` _output
          (:`Is Valid`
            (`InstancedStaticMeshComponent.UpdateInstanceTransform` _output _output_2 (`KismetMathLibrary.MakeTransform` (.location _outinstancetransform) (`KismetMathLibrary.MakeRotator` (`KismetMathLibrary.Lerp` (.roll (.rotation _outinstancetransform)) 0.0 _alpha)) (.scale _outinstancetransform)) false true false))))
      (:`Finished`
        (`KismetArrayLibrary.Array_Remove` (`self.ActiveAnimation`))
        (`KismetArrayLibrary.Array_Remove` (`self.ActiveKey`))
        (`self.CheckForActiveKey`)))))

(fn `Play Note`
  (params (note :type Integer) (keyType :type String))
  (`self.PlaySound` note keyType))

(fn `UserConstructionScript`
  ;[0.372 1 0.3197] Black keys style
  (bind _returnvalue (`AddComponent|NODE_AddInstancedStaticMeshComponent-2`))
  ;[0.3047 1 0.2011] White keys style
  (bind _returnvalue_2 (`AddComponent|NODE_AddInstancedStaticMeshComponent-0`))
  (for _index (range 1 (+ (`self.Size`) 1))
    (for _index_2 (range 12)
      (bind _output_get (set `self.CurrentIndex` _index_2))
      (if (== (mod (`self.CurrentIndex`) 12) 5)
        (bind _returnvalue_3 (/ (* _output_get (`self.HorizontalKeyDist`)) 2.0))
        (`InstancedStaticMeshComponent.AddInstance` _returnvalue_2 (`KismetMathLibrary.MakeTransform` (`KismetMathLibrary.MakeVector` (+ (+ _returnvalue_3 (/ (`self.HorizontalKeyDist`) 2.0)) (`self.H_Step`))) (`self.WhiteKeysRotation`) (`self.WhiteKeysSize`)))
        (set `self.H_Step` (+ (`self.H_Step`) (/ (`self.HorizontalKeyDist`) 2.0)))
        (set `self.V_Step` 1)
        (`KismetArrayLibrary.Array_Add` (`self.WhiteKeysArray`) _returnvalue_2)
        (else
          (bind _returnvalue_4 (* (mod (- _index_2 (`self.V_Step`)) 2) (`self.VerticalKeyDist`)))
          (if (!= _returnvalue_4 0.0)
            (bind _returnvalue_5 (+ _returnvalue_3 (`self.H_Step`)))
            ;[1 1 1] Black keys
            (`InstancedStaticMeshComponent.AddInstance` _returnvalue (`KismetMathLibrary.MakeTransform` (`KismetMathLibrary.MakeVector` _returnvalue_5 0.0 _returnvalue_4) (`self.BlackKeysRotation`) (`self.BlackKeysSize`)))
            (`KismetArrayLibrary.Array_Add` (`self.BlackKeysArray`) _returnvalue)
            (else
              (`InstancedStaticMeshComponent.AddInstance` _returnvalue_2 (`KismetMathLibrary.MakeTransform` (`KismetMathLibrary.MakeVector` _returnvalue_5 0.0 _returnvalue_4) (`self.WhiteKeysRotation`) (`self.WhiteKeysSize`)))
              (`KismetArrayLibrary.Array_Add` (`self.WhiteKeysArray`) _returnvalue_2))))))
    (set `self.V_Step` 0)
    (set `self.H_Step` (* (* _index 7) (`self.HorizontalKeyDist`)))))