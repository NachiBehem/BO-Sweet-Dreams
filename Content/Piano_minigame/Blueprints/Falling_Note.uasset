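; Falling note actor for the piano minigame that drops at constant speed along its negative up vector.
; On overlap it stores the other actor as its target and notifies the piano reference set through SetPianoRef.
; When the overlap ends it reports a miss and destroys itself.
; PlayerHitNote destroys the note and returns a precision score, deducting the truncated Y distance to the target from a maximum.
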(event `self.ReceiveActorBeginOverlap`
  (params (OtherActor :type "Actor Object Reference"))
  (set `self.FallingTarget` OtherActor)
  (message `/Game/Piano_minigame/Blueprints/I_Piano.FallingNoteEnter` (`self.BP_Piano_REF`) self))

(event `self.ReceiveActorEndOverlap`
  (params (OtherActor :type "Actor Object Reference"))
  (message `/Game/Piano_minigame/Blueprints/I_Piano.FallingNoteMiss` (`self.BP_Piano_REF`) self)
  (`self.K2_DestroyActor`))

(event `self.ReceiveTick`
  (params (DeltaSeconds :type "Float (single-precision)"))
  (`self.K2_SetActorLocation` (+ (* (`self.GetActorUpVector`) (* DeltaSeconds -30.0)) (`self.K2_GetActorLocation`))))

(fn `PlayerHitNote`
  (returns (Score :type Integer))
  (bind (_returnvalue_x _returnvalue_y) (`KismetMathLibrary.BreakVector` (`self.K2_GetActorLocation`)))
  (bind (_returnvalue_x_2 _returnvalue_y_2) (`KismetMathLibrary.BreakVector` (`self.K2_GetActorLocation` (`self.FallingTarget`))))
  (`self.K2_DestroyActor`)
  (return (- 10 (`KismetMathLibrary.FTrunc` (`KismetMathLibrary.Abs` (- _returnvalue_y_2 _returnvalue_y))))))

(fn `SetPianoRef`
  (params (Piano :type "/Game/Piano_minigame/BP_Piano Object Reference"))
  (set `self.BP_Piano_REF` Piano))

(fn `UserConstructionScript`
  (set `self.Height` (.z (`KismetSystemLibrary.GetComponentBounds` (`self.Sphere`)))))