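; Piano minigame audio processor actor that displays a row of eight note markers and spawns falling notes by key.
; The construction script builds the markers with dynamic transparent materials, which press and release functions recolor, fade and rescale as feedback.
; SpawnNote creates a Falling_Note, passes it the key and piano reference, and positions it through the note's own location lookup.
; StopTrack stops the audio, while StartTrack is empty.
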(event `SpawnNote`
  (params (key :type Integer))
  (bind _returnvalue (`self.GetTransform`))
  (bind (_returnvalue_x _returnvalue_y _returnvalue_z) (`KismetMathLibrary.BreakVector` (* (.scale _returnvalue) (`self.NoteScale`))))
  (bind _returnvalue_2 (`|SpawnActorFromClass` "/Game/Piano_minigame/Blueprints/Falling_Note.Falling_Note_C" _returnvalue "AlwaysSpawn" "OverrideRootScale" null null))
  (set `/Game/Piano_minigame/Blueprints/Falling_Note.Id` key _returnvalue_2)
  (set `/Game/Piano_minigame/Blueprints/Falling_Note.BP_Piano_REF` (`self.Piano_REF`) _returnvalue_2)
  (bind _returnvalue_x_2 (`KismetMathLibrary.BreakVector` (`self.GetActorScale3D` _returnvalue_2)))
  (bind (_returnvalue_x_3 _returnvalue_y_2 _returnvalue_z_2) (`KismetMathLibrary.BreakVector` (`self.K2_GetActorLocation` _returnvalue_2)))
  (`self.K2_SetActorTransform` _returnvalue_2 (`KismetMathLibrary.MakeTransform` (+ (+ (`KismetMathLibrary.MakeVector` (+ (- (* key (* (`self.Distance`) _returnvalue_x_2)) (* (`self.offset`) _returnvalue_x_2)) _returnvalue_x_3) _returnvalue_y_2 _returnvalue_z_2) 0.0) (* (`self.GetActorUpVector` _returnvalue_2) 100.0)) (`KismetMathLibrary.ComposeRotators` (`self.NoteRotation`) (.rotation _returnvalue)) (`KismetMathLibrary.MakeVector` _returnvalue_x _returnvalue_y (* _returnvalue_z 3.0))) false false))

(fn `Note Pressed`
  (params (note :type Integer))
  (bind _output (`|GetArrayItem` (`self.NoteArray`) note))
  (bind _output_2 (`|GetArrayItem` (`self.DynMaterial`) note))
  (`MaterialInstanceDynamic.SetScalarParameterValue` _output_2 "Alpha" 1.0)
  (`MaterialInstanceDynamic.SetVectorParameterValue` _output_2 "Base" (`self.PressedColor`))
  (`SceneComponent.K2_SetRelativeTransform` _output (`KismetMathLibrary.MakeTransform` (.location (`SceneComponent.GetRelativeTransform` _output)) (.rotation (`SceneComponent.GetRelativeTransform` _output)) (- (.scale (`SceneComponent.GetRelativeTransform` _output)) 0.1)) false false))

(fn `NoteReleased`
  (params (Note :type Integer))
  (bind _output (`|GetArrayItem` (`self.NoteArray`) Note))
  (bind _output_2 (`|GetArrayItem` (`self.DynMaterial`) Note))
  (`MaterialInstanceDynamic.SetScalarParameterValue` _output_2 "Alpha" 0.6)
  (`MaterialInstanceDynamic.SetVectorParameterValue` _output_2 "Base" (`self.BaseColor`))
  (`SceneComponent.K2_SetRelativeTransform` _output (`KismetMathLibrary.MakeTransform` (.location (`SceneComponent.GetRelativeTransform` _output)) (.rotation (`SceneComponent.GetRelativeTransform` _output)) (`self.NoteScale`)) true false))

(fn `StartTrack`
  (params (Piano :type "/Game/Piano_minigame/Blueprints/BP_PianoKeyboard Object Reference")))

(fn `StopTrack`
  (`AudioComponent.Stop` (`self.Audio`)))

(fn `UserConstructionScript`
  (locals (NewLocalVar_0 :type "Vector Structure" :default (1.0 1.0 1.0)))
  (for _index (range 8)
    (bind _returnvalue (`AddComponent|NODE_AddStaticMeshComponent-0` :`RelativeTransform` (`KismetMathLibrary.MakeTransform` (`KismetMathLibrary.MakeVector` 0.0 (- (* _index (`self.Distance`)) (`self.offset`)) -10.0) (`self.NoteRotation`) (`self.NoteScale`))))
    (`KismetArrayLibrary.Array_Add` (`self.NoteArray`) _returnvalue)
    (bind _returnvalue_2 (`PrimitiveComponent.CreateDynamicMaterialInstance` _returnvalue 0 "/Game/Piano_minigame/Material/M_Playable_Transparent.M_Playable_Transparent" "None"))
    (`KismetArrayLibrary.Array_Add` (`self.DynMaterial`) _returnvalue_2)))