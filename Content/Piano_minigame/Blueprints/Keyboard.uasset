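; Piano keyboard for the piano minigame, with key meshes for three octaves addressed by MIDI-style note number.
; BeginPlay builds a note-to-mesh map that goes unused, while GetKeyMesh repeats the lookup as a switch, with sharps sharing the natural key's mesh.
; NotePressed only prints a debug string.
; NoteReleased runs a timed MoveComponentTo on the key toward its current location, so no key press animation is functional yet.
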(event `self.ReceiveBeginPlay`
  (set `self.Keys` (`|MakeMap` 48.0 (`StaticMeshComponent.StaticMesh` (`self.c3`)) 49.0 (`StaticMeshComponent.StaticMesh` (`self.c3#`)) 50.0 (`StaticMeshComponent.StaticMesh` (`self.d3`)) 51.0 (`StaticMeshComponent.StaticMesh` (`self.d3#`)) 52.0 (`StaticMeshComponent.StaticMesh` (`self.e3`)) 53.0 (`StaticMeshComponent.StaticMesh` (`self.f3`)) 54.0 (`StaticMeshComponent.StaticMesh` (`self.f#3`)) 55.0 (`StaticMeshComponent.StaticMesh` (`self.g3`)) 56.0 (`StaticMeshComponent.StaticMesh` (`self.g3#`)) 57.0 (`StaticMeshComponent.StaticMesh` (`self.a3`)) 58.0 (`StaticMeshComponent.StaticMesh` (`self.a3#`)) 59.0 (`StaticMeshComponent.StaticMesh` (`self.b3`)) 60.0 (`StaticMeshComponent.StaticMesh` (`self.c4`)) 61.0 (`StaticMeshComponent.StaticMesh` (`self.c4#`)) 62.0 (`StaticMeshComponent.StaticMesh` (`self.d4`)) 63.0 (`StaticMeshComponent.StaticMesh` (`self.d4#`)) 64.0 (`StaticMeshComponent.StaticMesh` (`self.e4`)) 65.0 (`StaticMeshComponent.StaticMesh` (`self.f4`)) 66.0 (`StaticMeshComponent.StaticMesh` (`self.f4#`)) 67.0 (`StaticMeshComponent.StaticMesh` (`self.g4`)) 68.0 (`StaticMeshComponent.StaticMesh` (`self.g4#`)) 69.0 (`StaticMeshComponent.StaticMesh` (`self.a4`)) 70.0 (`StaticMeshComponent.StaticMesh` (`self.a4#`)) 71.0 (`StaticMeshComponent.StaticMesh` (`self.b4`)) 72.0 (`StaticMeshComponent.StaticMesh` (`self.c5`)) 73.0 (`StaticMeshComponent.StaticMesh` (`self.c5#`)) 74.0 (`StaticMeshComponent.StaticMesh` (`self.d5`)) 75.0 (`StaticMeshComponent.StaticMesh` (`self.d5#`)) 76.0 (`StaticMeshComponent.StaticMesh` (`self.e5`)) 77.0 (`StaticMeshComponent.StaticMesh` (`self.f5`)) 78.0 (`StaticMeshComponent.StaticMesh` (`self.f5#`)) 79.0 (`StaticMeshComponent.StaticMesh` (`self.g5`)) 80.0 (`StaticMeshComponent.StaticMesh` (`self.g5#`)) 81.0 (`StaticMeshComponent.StaticMesh` (`self.a5`)) 82.0 (`StaticMeshComponent.StaticMesh` (`self.a5#`)) 83.0 (`StaticMeshComponent.StaticMesh` (`self.b5`)) :!type "Float (single-precision)")))

(event `NotePressed`
  (params (note :type Integer))
  (`KismetSystemLibrary.PrintString` "Hello"))

(event `NoteReleased`
  (params (Note :type Integer))
  (bind _output_get (`self.Get Key Mesh` Note))
  (`KismetSystemLibrary.MoveComponentTo` _output_get (`SceneComponent.RelativeLocation` _output_get) (struct) false false 0.5))

(fn `Get Key Mesh`
  (params (Selection :type Integer))
  (returns (Output_Get :type "StaticMeshComponent Object Reference"))
  (switch `int` Selection
    (:`48`
      (set `self.KeyToTrigger` (`self.c3`)))
    (:`49`
      (set `self.KeyToTrigger` (`self.c3#`)))
    (:`50`
      (set `self.KeyToTrigger` (`self.d3`)))
    (:`51`
      (set `self.KeyToTrigger` (`self.d3#`)))
    (:`52`
      (set `self.KeyToTrigger` (`self.e3`)))
    (:`53`
      (set `self.KeyToTrigger` (`self.f3`)))
    (:`54`
      (set `self.KeyToTrigger` (`self.f#3`)))
    (:`55`
      (set `self.KeyToTrigger` (`self.g3`)))
    (:`56`
      (set `self.KeyToTrigger` (`self.g3#`)))
    (:`57`
      (set `self.KeyToTrigger` (`self.a3`)))
    (:`58`
      (set `self.KeyToTrigger` (`self.a3#`)))
    (:`59`
      (set `self.KeyToTrigger` (`self.b3`)))
    (:`60`
      (set `self.KeyToTrigger` (`self.c4`)))
    (:`61`
      (set `self.KeyToTrigger` (`self.c4#`)))
    (:`62`
      (set `self.KeyToTrigger` (`self.d4`)))
    (:`63`
      (set `self.KeyToTrigger` (`self.d4#`)))
    (:`64`
      (set `self.KeyToTrigger` (`self.e4`)))
    (:`65`
      (set `self.KeyToTrigger` (`self.f4`)))
    (:`66`
      (set `self.KeyToTrigger` (`self.f4#`)))
    (:`67`
      (set `self.KeyToTrigger` (`self.g4`)))
    (:`68`
      (set `self.KeyToTrigger` (`self.g4#`)))
    (:`69`
      (set `self.KeyToTrigger` (`self.a4`)))
    (:`70`
      (set `self.KeyToTrigger` (`self.a4#`)))
    (:`71`
      (set `self.KeyToTrigger` (`self.b4`)))
    (:`72`
      (set `self.KeyToTrigger` (`self.c5`)))
    (:`73`
      (set `self.KeyToTrigger` (`self.c5#`)))
    (:`74`
      (set `self.KeyToTrigger` (`self.d5`)))
    (:`75`
      (set `self.KeyToTrigger` (`self.d5#`)))
    (:`76`
      (set `self.KeyToTrigger` (`self.e5`)))
    (:`77`
      (set `self.KeyToTrigger` (`self.f5`)))
    (:`78`
      (set `self.KeyToTrigger` (`self.f5#`)))
    (:`79`
      (set `self.KeyToTrigger` (`self.g5`)))
    (:`80`
      (set `self.KeyToTrigger` (`self.g5#`)))
    (:`81`
      (set `self.KeyToTrigger` (`self.a5`)))
    (:`82`
      (set `self.KeyToTrigger` (`self.a5#`)))
    (:`83`
      (set `self.KeyToTrigger` (`self.b5`))))
  (return (`self.KeyToTrigger`)))

(fn `UserConstructionScript`)