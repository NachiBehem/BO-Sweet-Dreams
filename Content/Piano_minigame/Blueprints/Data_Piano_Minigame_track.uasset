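; Data object for a piano minigame track, exposing the track, its preview sound and its difficulty through getter functions.
; All three getters read from a single Data variable.
; The preview and track are returned as stored, while the difficulty enum is converted to a string.
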(fn `GetDifficultyString`
  (returns (Difficulty_string :type String))
  (return (`|GetEnumeratorNameAsString` (`.Difficulty_10_6AC61B1643FE6F8BB4C8C3B88CA46F64` (break `/Game/Piano_minigame/Blueprints/Piano_minigame_track_Struct` (`self.Data`))))))

(fn `GetSoundWave`
  (returns (Soundwave :type "SoundWave Object Reference"))
  (return (`.Preview_13_BAD5B208447A95C84EAFFC932710E4C2` (break `/Game/Piano_minigame/Blueprints/Piano_minigame_track_Struct` (`self.Data`)))))

(fn `GetTrack`
  (returns (TrackSequencer :type "LevelSequence Object Reference"))
  (return (`.Track_6_FD3B28DB4B7D502378B5CD9C0686CA91` (break `/Game/Piano_minigame/Blueprints/Piano_minigame_track_Struct` (`self.Data`)))))