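; BP_SelectLevel is an interaction point that opens the level selection menu.
; Its Scene component and children are hidden at BeginPlay, while Box overlaps add and remove an InputRequest prompt widget without filtering the overlapping actor.
; OnPlayerInteract creates the Levels_menu widget for player controller 0, switches input to UI only and shows the mouse cursor.
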(event `self.ReceiveBeginPlay`
  (`SceneComponent.SetVisibility` (`self.Scene`) false true))

(event `self.Box.OnComponentBeginOverlap`
  (params (OverlappedComponent :type "PrimitiveComponent Object Reference") (OtherActor :type "Actor Object Reference") (OtherComp :type "PrimitiveComponent Object Reference") (OtherBodyIndex :type Integer) (bFromSweep :type Boolean) (SweepResult :type "HitResult Structure (by ref)"))
  (bind _returnvalue (`|CreateWidget` "/Game/BP/InputRequest.InputRequest_C"))
  (`UserWidget.AddToViewport` _returnvalue 0))

(event `self.Box.OnComponentEndOverlap`
  (params (OverlappedComponent :type "PrimitiveComponent Object Reference") (OtherActor :type "Actor Object Reference") (OtherComp :type "PrimitiveComponent Object Reference") (OtherBodyIndex :type Integer))
  (`Widget.RemoveFromParent` (stale `self.Box.OnComponentBeginOverlap` _returnvalue)))

(event `/Game/BaseIteractableInterface.On Player Interact`
  (params (Player :type "/Game/ThirdPersonBP/ThirdPersonCharacter Object Reference"))
  (bind _returnvalue (`GameplayStatics.GetPlayerController` 0))
  (bind _returnvalue_2 (`|CreateWidget` "/Game/HUD/SelectLevel/Widget/Levels_menu.Levels_menu_C" _returnvalue))
  (`UserWidget.AddToViewport` _returnvalue_2 0)
  (`WidgetBlueprintLibrary.SetInputMode_UIOnlyEx` _returnvalue _returnvalue_2)
  (set `PlayerController.bShowMouseCursor` true _returnvalue))

(fn `UserConstructionScript`)