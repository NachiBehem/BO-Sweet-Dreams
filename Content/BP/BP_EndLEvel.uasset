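; BP_EndLEvel is a box trigger that runs the end sequence of the village level when a player-tagged actor overlaps it.
; It spawns BP_Lupo_pH at a fixed location, flags EndVillage on Alice and applies damage to Alice every half second until Alice's Health reads 100 or more.
; It then records the first-level milestone and sets dialogue progression to "After Nightmare" in AliceGameInstance.
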(event `self.Box.OnComponentBeginOverlap`
  (params (OverlappedComponent :type "PrimitiveComponent Object Reference") (OtherActor :type "Actor Object Reference") (OtherComp :type "PrimitiveComponent Object Reference") (OtherBodyIndex :type Integer) (bFromSweep :type Boolean) (SweepResult :type "HitResult Structure (by ref)"))
  (if (`self.ActorHasTag` OtherActor "player")
    (`|SpawnActorFromClass` "/Game/BP/BP_Lupo_pH.BP_Lupo_pH_C" (`KismetMathLibrary.MakeTransform` (8325.137695 -16285.527344 4925.961914) (struct) (1.5 1.5 1.5)) "Undefined" "OverrideRootScale" null null)
    (bind _returnvalue (`GameplayStatics.GetActorOfClass` "/Game/Alice/Toon/Blueprints/Alice.Alice_C"))
    (set `/Game/Alice/Toon/Blueprints/Alice.EndVillage` true _returnvalue)
    (`GameplayStatics.ApplyDamage` _returnvalue 25.0 null self :!label _label)
    (if (>= (`/Game/Alice/Toon/Blueprints/Alice.Health` _returnvalue) 100.0)
      (bind _asalice_game_instance (cast `/Game/Alice/AliceGameInstance` (`GameplayStatics.GetGameInstance`)))
      (set `/Game/Alice/AliceGameInstance.FirstLevelMilestone` 1 _asalice_game_instance)
      (set `/Game/Alice/AliceGameInstance.Dialogue Progression` "After Nightmare" _asalice_game_instance)
      (else
        (`KismetSystemLibrary.Delay` 0.5)
        (goto _label)))))

(fn `UserConstructionScript`)