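; Trigger actor that ends the game or demo when an actor tagged "player" overlaps its Box, despite its level-switch name.
; It clears the TheRuins flag in the AliceGameInstance level progression struct and plays a sound.
; It then shows TheEnd widget with UI-only input, cursor and button focus, and pauses the game.
; The level-open call to M_EncounterRuinedVillage is left unconnected and never runs.
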(event `self.Box.OnComponentBeginOverlap`
  (params (OverlappedComponent :type "PrimitiveComponent Object Reference") (OtherActor :type "Actor Object Reference") (OtherComp :type "PrimitiveComponent Object Reference") (OtherBodyIndex :type Integer) (bFromSweep :type Boolean) (SweepResult :type "HitResult Structure (by ref)"))
  (bind _returnvalue (`GameplayStatics.GetPlayerController` 0))
  (if (`self.ActorHasTag` OtherActor "player")
    (setmembers `/Game/Alice/LevelProgression` :`StructRef` (`/Game/Alice/AliceGameInstance.Level Progression` (cast `/Game/Alice/AliceGameInstance` (`GameplayStatics.GetGameInstance`) :!pure true)) :`The Ruins` false)
    (`GameplayStatics.PlaySound2D` "/Game/SOUND_EFFECTS/Books_on_Shelf/SC_Book_OUT_Shelf.SC_Book_OUT_Shelf" 1.0 1.0 0.0 null null)
    (bind _returnvalue_2 (`|CreateWidget` "/Game/Alerts/TheEnd.TheEnd_C" _returnvalue))
    (`UserWidget.AddToViewport` _returnvalue_2 0)
    (`WidgetBlueprintLibrary.SetInputMode_UIOnlyEx` _returnvalue _returnvalue_2)
    (set `PlayerController.bShowMouseCursor` true _returnvalue)
    (bind _button_55 (`/Game/Alerts/TheEnd.Button_55` _returnvalue_2))
    (`Widget.SetKeyboardFocus` _button_55)
    (`Widget.SetFocus` _button_55)
    (`GameplayStatics.SetGamePaused` true)
    (else
      (`KismetSystemLibrary.PrintString` "NO"))))

(fn `UserConstructionScript`)