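; Audio processor Blueprint for the piano minigame, sketching Quartz-based, beat-synced music playback that is currently inactive.
; An unconnected chain creates a 4/4 "Beat" clock, sets its tempo, plays audio quantized to quarter notes and subscribes to all quantization events.
; The music callback resumes the clock once playback is queued.
; BeginPlay is empty, and the clock event switches on quantization type without acting.
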(event `self.ReceiveBeginPlay`)

(event `OnTickMusic`
  (params (EventType :type "EQuartzCommandDelegateSubType Enum" :default "CommandOnFailedToQueue") (Name :type Name))
  (switch `EQuartzCommandDelegateSubType` EventType
    (:`CommandOnQueued`
      (`QuartzClockHandle.ResumeClock` (`self.clock`)))))

(event `allclock event`
  (params (ClockName :type Name) (QuantizationType :type "EQuartzCommandQuantization Enum" :default "Bar") (NumBars :type Integer) (Beat :type Integer) (BeatFraction :type "Float (double-precision)"))
  (switch `EQuartzCommandQuantization` QuantizationType))

(fn `Audio_Controller_BP_AutoGenFunc`
  (params (ClockName :type Name) (QuantizationType :type "EQuartzCommandQuantization Enum" :default "Bar") (NumBars :type Integer) (Beat :type Integer) (BeatFraction :type "Float (double-precision)")))

(fn `UserConstructionScript`)